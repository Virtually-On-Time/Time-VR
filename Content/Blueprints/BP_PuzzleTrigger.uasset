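; BP_PuzzleTrigger is an overlap trigger that detects when the correct puzzle item is placed on it.
; On BeginPlay it caches the VRGameMode.
; When an overlapping actor is exactly a BP_PuzzleItem and its PuzzleID matches the trigger's PuzzleKey, it locks the item in place and notifies the game mode through TriggerPuzzle with that key.
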(event EventBeginPlay
  ;[1 1 1] Find reference to VR_GameMode
  (bind _asvrgame_mode (Utilities|Casting|CastToVRGameMode (Game|GetGameMode)))
  (Variables|Default|SetVRGameMode _asvrgame_mode))

(event Collision|EventActorBeginOverlap
  (params (OtherActor :type Actor%20Object%20Reference))
  ;[1 1 1] Check if overlaped actor is puzzle item
  (if (== "/Game/Blueprints/BP_PuzzleItem.BP_PuzzleItem_C" (Utilities|GetClass OtherActor))
    (bind _asbp_puzzle_item (Utilities|Casting|CastToBP_PuzzleItem OtherActor))
    ;[1 1 1] Check that puzzle item is correct
    (if (== (Variables|/Game/Blueprints/BP_PuzzleItem.BP_PuzzleItem_C|GetPuzzleID _asbp_puzzle_item) (Variables|Default|GetPuzzleKey))
      (Development|PrintString "Puzzle success!")
      ;[1 1 1] Inform other blueprints
      (Default|LockinPlace _asbp_puzzle_item)
      (Default|TriggerPuzzle (Variables|Default|GetVRGameMode) (Variables|Default|GetPuzzleKey)))))

(event EventTick
  (params (DeltaSeconds :type Float%20%28single-precision%29)))

(fn ConstructionScript)