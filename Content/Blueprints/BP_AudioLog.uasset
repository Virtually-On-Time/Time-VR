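; BP_AudioLog is an audio log actor that the player starts and stops by touching it with a BP_HandController.
; Audio is stopped on BeginPlay, then each hand controller overlap toggles it and swaps the visibility of the play and pause icon components.
; Despite the pause icon, toggling off fully stops the audio, so the next touch replays it from the beginning.
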(event EventBeginPlay
  ;[1 1 1] Prevent Audio form playing on Start
  (Audio|Components|Audio|Stop (Variables|Default|GetAudio)))

(event Collision|EventActorBeginOverlap
  (params (OtherActor :type Actor%20Object%20Reference))
  (bind _audio (Variables|Default|GetAudio))
  (bind _spr_play (Variables|Default|GetSPR_Play))
  (bind _spr_pause (Variables|Default|GetSPR_Pause))
  ;[1 1 1] If Player overlaps with AudioLog
  (if (== (Utilities|GetClass OtherActor) "/Game/Blueprints/BP_HandController.BP_HandController_C")
    ;[1 1 1] Play / Pause Audio
    (if (Audio|Components|Audio|IsPlaying (Variables|Default|GetAudio))
      (Audio|Components|Audio|Stop _audio)
      ;[1 1 1] Update Icon Visibility
      (Rendering|SetVisibility _spr_play true false)
      (Rendering|SetVisibility _spr_pause false false)
      (else
        (Audio|Components|Audio|Play _audio 0.0)
        (Rendering|SetVisibility _spr_pause true false)
        (Rendering|SetVisibility _spr_play false false)))))

(event EventTick
  (params (DeltaSeconds :type Float%20%28single-precision%29)))

(fn ConstructionScript)