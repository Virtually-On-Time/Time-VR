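; BP_AudioTablet is a VR audio-log tablet that plays one of four recordings and can advance game discoveries.
; Overlap triggers act as play, previous and next buttons, firing on release, with HeldId allowing one press at a time.
; Track changes clamp the index, update the label and start playback.
; When audio finishes, Character and index gate delayed GameMode virus or weapon interactions, though the Captain's weapon threshold exceeds the clamped range.
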(event OnComponentBeginOverlap(PrevTrigger)
  (params (OverlappedComponent :type Primitive%20Component%20Object%20Reference) (OtherActor :type Actor%20Object%20Reference) (OtherComp :type Primitive%20Component%20Object%20Reference) (OtherBodyIndex :type Integer) (bFromSweep :type Boolean) (SweepResult :type Hit%20Result%20Structure%20%28by%20ref%29))
  ;[1 1 1] Tablet button touched
  (if (== (Variables|Default|GetHeldId) 0)
    (Development|PrintString "_2")
    (Variables|Default|SetHeldId 2)))

(event OnComponentBeginOverlap(NextTrigger)
  (params (OverlappedComponent :type Primitive%20Component%20Object%20Reference) (OtherActor :type Actor%20Object%20Reference) (OtherComp :type Primitive%20Component%20Object%20Reference) (OtherBodyIndex :type Integer) (bFromSweep :type Boolean) (SweepResult :type Hit%20Result%20Structure%20%28by%20ref%29))
  ;[1 1 1] Tablet button touched
  (if (== (Variables|Default|GetHeldId) 0)
    (Development|PrintString "_3")
    (Variables|Default|SetHeldId 3)))

(event OnComponentBeginOverlap(PlayTrigger)
  (params (OverlappedComponent :type Primitive%20Component%20Object%20Reference) (OtherActor :type Actor%20Object%20Reference) (OtherComp :type Primitive%20Component%20Object%20Reference) (OtherBodyIndex :type Integer) (bFromSweep :type Boolean) (SweepResult :type Hit%20Result%20Structure%20%28by%20ref%29))
  ;[1 1 1] Tablet button touched
  (if (== (Variables|Default|GetHeldId) 0)
    (Development|PrintString "_1")
    (Variables|Default|SetHeldId 1)))

(event OnComponentEndOverlap(NextTrigger)
  (params (OverlappedComponent :type Primitive%20Component%20Object%20Reference) (OtherActor :type Actor%20Object%20Reference) (OtherComp :type Primitive%20Component%20Object%20Reference) (OtherBodyIndex :type Integer))
  ;[1 1 1] Tablet button released
  (if (== 3 (Variables|Default|GetHeldId))
    (CallFunction|ATNext)
    (Variables|Default|SetHeldId 0)))

(event OnComponentEndOverlap(PlayTrigger)
  (params (OverlappedComponent :type Primitive%20Component%20Object%20Reference) (OtherActor :type Actor%20Object%20Reference) (OtherComp :type Primitive%20Component%20Object%20Reference) (OtherBodyIndex :type Integer))
  ;[1 1 1] Tablet button released
  (if (== 1 (Variables|Default|GetHeldId))
    (CallFunction|ATPlay)
    (Variables|Default|SetHeldId 0)))

(event OnComponentEndOverlap(PrevTrigger)
  (params (OverlappedComponent :type Primitive%20Component%20Object%20Reference) (OtherActor :type Actor%20Object%20Reference) (OtherComp :type Primitive%20Component%20Object%20Reference) (OtherBodyIndex :type Integer))
  ;[1 1 1] Tablet button released
  (if (== 2 (Variables|Default|GetHeldId))
    (CallFunction|ATPrev)
    (Variables|Default|SetHeldId 0)))

(event OnAudioFinished(Audio)
  (Development|PrintString (Utilities|String|Append "Audio Finished: " (Utilities|String|EnumtoString (Variables|Default|GetCharacter))))
  (Utilities|FlowControl|Sequence
    (:then_0
      (switch Utilities|FlowControl|Switch|SwitchonEN_Characters (Variables|Default|GetCharacter)
        (:NewEnumerator1
          ;[1 1 1] Discover Weapon Logic
          (if (> (Variables|Default|GetAudioTrackIndex) 3)
            (Utilities|FlowControl|Delay 1.0)
            (Default|TriggerInteraction (Variables|Default|GetGameMode) 5)))))
    (:then_1
      (switch Utilities|FlowControl|Switch|SwitchonEN_Characters (Variables|Default|GetCharacter)
        (:NewEnumerator0
          ;[1 1 1] Discover Virus Logic
          (if (> (Variables|Default|GetAudioTrackIndex) 2)
            (Utilities|FlowControl|Delay 1.0)
            (Default|TriggerInteraction (Variables|Default|GetGameMode) 4)))
        (:NewEnumerator1
          (if (> (Variables|Default|GetAudioTrackIndex) 2)
            _))))))

(event Custom|AT_Play
  ;[1 1 1] Play/Pause
  (if (not (Audio|Components|Audio|IsPlaying (Variables|Default|GetAudio)))
    (Development|PrintString "PLAY")
    (Audio|Components|Audio|Play (Variables|Default|GetAudio) 0.0)))

(event Custom|AT_Next
  ;[1 1 1] Set track
  (Development|PrintString "PREV")
  (bind _result (Math|Integer|IncrementInt (Variables|Default|GetAudioTrackIndex))
    (:%20%20
      (Variables|Default|SetAudioTrackIndex (Math|Integer|Clamp(Integer) _result 0 3))
      (CallFunction|UpdateText)
      (bind _audiofile (CallFunction|GetAudioFile))
      (Audio|Components|Audio|SetSound (Variables|Default|GetAudio) _audiofile)
      (CallFunction|ATPlay))))

(event Custom|AT_Prev
  ;[1 1 1] Set track
  (Development|PrintString "NEXT")
  (bind _result (Math|Integer|DecrementInt (Variables|Default|GetAudioTrackIndex))
    (:%20%20
      (Variables|Default|SetAudioTrackIndex (Math|Integer|Clamp(Integer) _result 0 3))
      (CallFunction|UpdateText)
      (bind _audiofile (CallFunction|GetAudioFile))
      (Audio|Components|Audio|SetSound (Variables|Default|GetAudio) _audiofile)
      (CallFunction|ATPlay))))

(event Custom|Update%20text
  ;[1 1 1] Update track index
  (Rendering|Components|TextRender|SetText (Variables|Default|GetTextAudioIndex) (Utilities|Text|ToText(String) (Utilities|String|Append "Audio log " (Utilities|String|ToString(Integer) (+ (Variables|Default|GetAudioTrackIndex) 1))))))

(event EventBeginPlay
  ;[1 1 1] Find reference to VR_GameMode
  (bind _asvrgame_mode (Utilities|Casting|CastToVRGameMode (Game|GetGameMode)))
  (Variables|Default|SetGameMode _asvrgame_mode)
  (Variables|Default|SetAudioTrackIndex 0)
  (bind _audiofile (CallFunction|GetAudioFile))
  (Audio|Components|Audio|SetSound (Variables|Default|GetAudio) _audiofile))

(event Collision|EventActorBeginOverlap
  (params (OtherActor :type Actor%20Object%20Reference)))

(event EventTick
  (params (DeltaSeconds :type Float%20%28single-precision%29)))

(fn ConstructionScript)

(fn GetAudioFile
  (return (Utilities|Select :Index (Variables|Default|GetAudioTrackIndex) :Option%200 "/Game/Audio/Giovani/GE_01.GE_01" :Option%201 "/Game/Audio/Giovani/GE_02.GE_02" :Option%202 "/Game/Audio/Giovani/GE_03.GE_03" :Option%203 "/Game/Audio/Giovani/GE_04.GE_04")))